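; Player 1 actor for a versus game, which moves between three lanes (UP, MID, DOWN) by teleporting along X.
; Attack and Dodge events each set a one-second state flag: attacking drives the baseball bat's rotation through a timeline, while dodging temporarily shifts the actor along Y.
; Tick polls PuzzleGameMode and, while P2WIN is true, repeatedly shatters the destructible component and spawns an emitter at the Lioncub's location.
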(event Custom|PositionUP
  (bind _returnvalue (Transformation|GetActorLocation))
  (if (not (Utilities|Enum|Equal(Enum) (Variables|Default|GetPOSITION) "UP"))
    (if (Utilities|Enum|Equal(Enum) (Variables|Default|GetPOSITION) "MID")
      (Variables|Default|SetPOSITION "UP")
      (else
        (Variables|Default|SetPOSITION "MID")))
    (Transformation|SetActorLocation (Math|Vector|MakeVector (+ (.x _returnvalue) 1e+02) (.y _returnvalue) (.z _returnvalue)) false true)))

(event Custom|Dodge
  (bind _returnvalue (Transformation|GetActorLocation))
  (bind _returnvalue_2 (Transformation|GetActorLocation))
  (Variables|Default|SetisDodging true)
  (Transformation|SetActorLocation (Math|Vector|MakeVector (.x _returnvalue_2) (+ (.y _returnvalue_2) -2e+02) (.z _returnvalue_2)) false true)
  (Utilities|FlowControl|Delay 1.0)
  (Variables|Default|SetisDodging false)
  (Transformation|SetActorLocation (Math|Vector|MakeVector (.x _returnvalue) (+ (.y _returnvalue) 2e+02) (.z _returnvalue)) false true))

(event Custom|Attack
  (bind _baseball_bat (Variables|Default|GetBaseball_Bat))
  (Variables|Default|SetisAttacking true)
  (Utilities|FlowControl|Sequence
    (:then_0
      (Utilities|FlowControl|Delay 1.0)
      (Variables|Default|SetisAttacking false))
    (:then_1
      (bind _newtrack_0 (Timeline|Timeline_0 PlayFromStart)
        (:Update
          (Transformation|SetWorldRotation _baseball_bat (* (Transformation|GetWorldRotation _baseball_bat) (* _newtrack_0 3.6e+02)) false false))))))

(event Custom|PositionDOWN
  (bind _returnvalue (Transformation|GetActorLocation))
  (if (not (Utilities|Enum|Equal(Enum) (Variables|Default|GetPOSITION) "DOWN"))
    (if (Utilities|Enum|Equal(Enum) (Variables|Default|GetPOSITION) "UP")
      (Variables|Default|SetPOSITION "MID")
      (else
        (Variables|Default|SetPOSITION "DOWN")))
    (Transformation|SetActorLocation (Math|Vector|MakeVector (+ (.x _returnvalue) -1e+02) (.y _returnvalue) (.z _returnvalue)) false true)))

(event EventBeginPlay)

(event Collision|EventActorBeginOverlap
  (params (OtherActor :type Actor%20Object%20Reference)))

(event EventTick
  (params (DeltaSeconds :type Float%20%28single-precision%29))
  (bind _lion_cub (Variables|Default|Getlion-cub))
  (bind _returnvalue (Transformation|GetWorldLocation _lion_cub))
  (bind _aspuzzle_game_mode (Utilities|Casting|CastToPuzzleGameMode (Game|GetGameMode)))
  (if (Variables|/Game/PuzzleBP/Blueprints/PuzzleGameMode.PuzzleGameMode_C|GetP2WIN _aspuzzle_game_mode)
    (Game|Damage|ApplyDamage (Variables|Default|GetDestructibleComponent) 99999.0 _returnvalue (Math|Vector|Normalize _returnvalue) 999999.0)
    (Effects|SpawnEmitteratLocation 0 _returnvalue)))

(fn ConstructionScript)