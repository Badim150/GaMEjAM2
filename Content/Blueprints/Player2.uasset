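; Player2 is a player actor that shifts between three lanes (UP, MID, DOWN) and attacks with a baseball bat.
; PositionUP and PositionDOWN step the POSITION state, stop at the outer lanes, and teleport the actor 100 units along world X.
; Attack restarts a timeline that, on each update, multiplies the bat's current world rotation by the track value times 360, rather than setting an absolute angle.
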(event Custom|PositionUP
  (bind _returnvalue (Transformation|GetActorLocation))
  (if (not (Utilities|Enum|Equal(Enum) (Variables|Default|GetPOSITION) "UP"))
    (if (Utilities|Enum|Equal(Enum) (Variables|Default|GetPOSITION) "MID")
      (Variables|Default|SetPOSITION "UP")
      (else
        (Variables|Default|SetPOSITION "MID")))
    (Transformation|SetActorLocation (Math|Vector|MakeVector (+ (.x _returnvalue) 1e+02) (.y _returnvalue) (.z _returnvalue)) false true)))

(event Custom|Attack
  (bind _baseball_bat (Variables|Default|GetBaseball_Bat))
  (bind _newtrack_0 (Timeline|Timeline_0 PlayFromStart)
    (:Update
      (Transformation|SetWorldRotation _baseball_bat (* (Transformation|GetWorldRotation _baseball_bat) (* _newtrack_0 3.6e+02)) false false))))

(event Custom|PositionDOWN
  (bind _returnvalue (Transformation|GetActorLocation))
  (if (not (Utilities|Enum|Equal(Enum) (Variables|Default|GetPOSITION) "DOWN"))
    (if (Utilities|Enum|Equal(Enum) (Variables|Default|GetPOSITION) "UP")
      (Variables|Default|SetPOSITION "MID")
      (else
        (Variables|Default|SetPOSITION "DOWN")))
    (Transformation|SetActorLocation (Math|Vector|MakeVector (+ (.x _returnvalue) -1e+02) (.y _returnvalue) (.z _returnvalue)) false true)))

(event EventBeginPlay)

(event Collision|EventActorBeginOverlap
  (params (OtherActor :type Actor%20Object%20Reference)))

(event EventTick
  (params (DeltaSeconds :type Float%20%28single-precision%29)))

(fn ConstructionScript)